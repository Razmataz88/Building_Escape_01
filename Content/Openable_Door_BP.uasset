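; Openable door actor that swings open and shut in response to OnOpen and OnClose events from its OpenDoor component or interface.
; It caches its starting rotation on BeginPlay, then a timeline's OpenAngle track adds yaw to that rotation each update.
; Closing reverses the same timeline, and a timeline event track plays the door lock sound at the actor's location.
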(event OnOpen(OpenDoor)
  (bind _openangle (Timeline|Timeline_0 Play)
    (:Update
      (Transformation|SetActorRotation (Math|Rotator|CombineRotators (Math|Rotator|MakeRotator 0.0 0.0 _openangle) (Variables|Default|Getinitial%20rotation))))
    (:Sound%20Timing
      (Audio|SpawnSoundatLocation "/Game/Audio/door-lock.door-lock" (Transformation|GetActorLocation)))))

(event OnClose(OpenDoor)
  (bind _openangle (Timeline|Timeline_0 Reverse)
    (:Update
      (Transformation|SetActorRotation (Math|Rotator|CombineRotators (Math|Rotator|MakeRotator 0.0 0.0 _openangle) (Variables|Default|Getinitial%20rotation))))
    (:Sound%20Timing
      (Audio|SpawnSoundatLocation "/Game/Audio/door-lock.door-lock" (Transformation|GetActorLocation)))))

(event EventBeginPlay
  (Variables|Default|Setinitial%20rotation (Transformation|GetActorRotation)))

(fn ConstructionScript)